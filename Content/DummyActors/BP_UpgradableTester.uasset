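; BP_UpgradableTester is a dummy interactable actor for testing the upgrade and resource systems, with debug prints.
; Interacting requests a one-level upgrade from the upgrade subsystem using the instigator's PlayerState resources, then spends next-level costs regardless of success.
; Interacting during an active upgrade shortens the timer by half the remaining time plus five seconds.
; Widget1's timer display binds to the upgradable component, while sphere overlaps toggle another widget.
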(event OnComponentBeginOverlap(Sphere)
  (params (OverlappedComponent :type Primitive%20Component%20Object%20Reference) (OtherActor :type Actor%20Object%20Reference) (OtherComp :type Primitive%20Component%20Object%20Reference) (OtherBodyIndex :type Integer) (bFromSweep :type Boolean) (SweepResult :type Hit%20Result%20Structure%20%28by%20ref%29))
  (Utilities|Casting|CastToCharacter OtherActor)
  (Rendering|SetVisibility (Variables|Default|GetWidget) true false))

(event OnComponentEndOverlap(Sphere)
  (params (OverlappedComponent :type Primitive%20Component%20Object%20Reference) (OtherActor :type Actor%20Object%20Reference) (OtherComp :type Primitive%20Component%20Object%20Reference) (OtherBodyIndex :type Integer))
  (Rendering|SetVisibility (Variables|Default|GetWidget) false false))

(event Custom|Upgradelevel
  (bind _returnvalue (Subsystems|GetUpgradeManagerSubsystem))
  (bind _returnvalue_2 (Subsystems|GetUpgradeManagerSubsystem))
  (bind _bp_upgradablecomponent (Variables|Default|GetBP_UpgradableComponent))
  (bind _bp_upgradablecomponent_2 (Variables|Default|GetBP_UpgradableComponent))
  (bind _returnvalue_3 (Class|UpgradableComponent|GetComponentId _bp_upgradablecomponent))
  (bind _returnvalue_4 (Class|UpgradableComponent|GetComponentId _bp_upgradablecomponent_2))
  (bind _resourcecosts (Class|UpgradeManagerSubsystem|GetNextLevelUpgradeCosts _returnvalue _returnvalue_4))
  (if (Class|UpgradeManagerSubsystem|IsUpgradeTimerActive _returnvalue_2 _returnvalue_3)
    (bind _output_get (Variables|Default|SetUpgradeReduction (- (/ (Class|UpgradeManagerSubsystem|GetUpgradeTimeRemaining _returnvalue_2 _returnvalue_3) -2.0) 5.0)))
    (bind _returnvalue_5 (Class|UpgradeManagerSubsystem|UpdateUpgradeTimer (Subsystems|GetUpgradeManagerSubsystem) _returnvalue_3 _output_get))
    (if (< _returnvalue_5 0.0)
      (Development|PrintString (Utilities|String|Append "Reduced upgrade time by " (Utilities|String|ToString(Float) (Variables|Default|GetUpgradeReduction)) " and upgrade was completed!") true true "(R=0.037764,G=1.000000,B=0.000000,A=1.000000)" 5.0 "")
      (else
        (Development|PrintString (Utilities|String|Append "Reduced Upgrade Time by: " (Utilities|String|ToString(Float) (Variables|Default|GetUpgradeReduction)) " Time Remaining until completeion: " (Utilities|String|ToString(Float) _returnvalue_5)) true true "(R=0.037764,G=1.000000,B=0.000000,A=1.000000)" 5.0 "")))
    (else
      (bind _ascharacter (Utilities|Casting|CastToCharacter (Variables|Default|GetInstigator_0)))
      (Variables|Default|SetInstigatorResourceSystem (Actor|GetComponentbyClass (Variables|/Script/Engine.Pawn|GetPlayerState _ascharacter) "/Script/Plugin_Development.ResourceSystemComponent"))
      (bind _returnvalue_6 (Class|UpgradeManagerSubsystem|UpgradeComponent (Subsystems|GetUpgradeManagerSubsystem) (Class|UpgradableComponent|GetComponentId (Variables|Default|GetBP_UpgradableComponent)) (Class|ResourceSystemComponent|GetAllResources (Actor|GetComponentbyClass (Variables|/Script/Engine.Pawn|GetPlayerState _ascharacter) "/Script/Plugin_Development.ResourceSystemComponent")) 1))
      (Development|PrintString (Utilities|String|Append "Attempted to start upgrading component. Success: " (Utilities|String|ToString(Boolean) _returnvalue_6) " Time to upgrade: " (Utilities|String|ToString(Float) (Class|UpgradeManagerSubsystem|GetUpgradeTimeRemaining (Subsystems|GetUpgradeManagerSubsystem) (Class|UpgradableComponent|GetComponentId (Variables|Default|GetBP_UpgradableComponent))))) true true "(R=0.795653,G=0.005113,B=1.000000,A=1.000000)" 5.0 "")
      (if true
        (bind _keys (Utilities|Map|Keys _resourcecosts))
        (for _array_element _keys
          (Class|ResourceSystemComponent|SpendResource (Variables|Default|GetInstigatorResourceSystem) _array_element (.Value (Utilities|Map|Find _resourcecosts _array_element)))
          (Utilities|IsValid (Class|ResourceManagerSubsystem|GetDefinition (Subsystems|GetResourceManagerSubsystem) _array_element)
            (:Is%20Valid
              (Development|PrintString (Utilities|String|Append "Spent resources for upgrade: " (Utilities|String|ToString(Name) _array_element) (Utilities|String|ToString(Text) (Variables|/Script/Plugin_Development.ResourceDefinition|GetDescription (Class|ResourceManagerSubsystem|GetDefinition (Subsystems|GetResourceManagerSubsystem) _array_element)))) true true "(R=0.795653,G=0.005113,B=1.000000,A=1.000000)" 5.0 ""))
            (:Is%20Not%20Valid
              (Development|PrintString "resource definition not valid" true true "(R=0.795653,G=0.005113,B=1.000000,A=1.000000)" 5.0 ""))))))))

(event EventBeginPlay
  (bind _aswbp_timer_display (Utilities|Casting|CastToWBP_TimerDisplay (UserInterface|GetWidget (Variables|Default|GetWidget1))))
  (Class|UpgradeTimerDisplay|BindUpgradableComponent _aswbp_timer_display (Class|UpgradableComponent|GetComponentId (Variables|Default|GetBP_UpgradableComponent))))

(event Collision|EventActorBeginOverlap
  (params (OtherActor :type Actor%20Object%20Reference)))

(event EventTick
  (params (DeltaSeconds :type Float%20%28single-precision%29)))

(event EventInteract
  (params (Instigator :type Actor%20Object%20Reference))
  (Variables|Default|SetInstigator_0 Instigator)
  (CallFunction|Upgradelevel))

(fn ConstructionScript)